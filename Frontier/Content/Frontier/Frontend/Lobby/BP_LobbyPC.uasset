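; BP_LobbyPC is the lobby player controller, bridging the lobby widget and the game mode.
; It creates WBP_Lobby on setup, pushes server info and player list updates into it, and removes it on EndPlay.
; Ready changes, map changes and game start are forwarded to BP_LobbyGM, with map changes sent as updated server settings.
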(event Custom|UpdatePlayerList
  (params (Players :type Array%20of%20Lobby%20Player%20Structures))
  (Default|UpdatePlayerList (Variables|Default|GetLobbyUI) Players))

(event Custom|UpdateServerInfo
  (params (Info :type Lobby%20Server%20Info%20Structure))
  (bind _lobbyui (Variables|Default|GetLobbyUI))
  (Variables|Default|SetServerInfo Info)
  (Utilities|IsValid _lobbyui
    (:Is%20Valid
      (CallFunction|SetLobbyUI _lobbyui))))

(event Custom|InitialSetup
  (bind _returnvalue (UserInterface|CreateWidget "/Game/Frontier/Frontend/Lobby/WBP_Lobby.WBP_Lobby_C"))
  (bind _output_get (Variables|Default|SetLobbyUI _returnvalue))
  (UserInterface|Viewport|AddtoViewport _output_get 0))

(event Custom|SetReady
  (params (Ready :type Boolean))
  (bind _asbp_lobby_gm (Utilities|Casting|CastToBP_LobbyGM (Game|GetGameMode)))
  (Default|SetPlayerReady _asbp_lobby_gm self Ready))

(event Custom|StartGame
  (bind _asbp_lobby_gm (Utilities|Casting|CastToBP_LobbyGM (Game|GetGameMode)))
  (Default|StartGame _asbp_lobby_gm))

(event Custom|UpdateMap
  (params (Map :type String))
  (bind _structout (Utilities|Struct|SetmembersinLobbyServerInfo (Variables|Default|GetServerInfo) Map))
  (bind _asbp_lobby_gm (Utilities|Casting|CastToBP_LobbyGM (Game|GetGameMode)))
  (Default|UpdateSettings _asbp_lobby_gm _structout))

(event EventEndPlay
  (params (EndPlayReason :type EEndPlayReason%20Enum :default "Destroyed"))
  (bind _lobbyui (Variables|Default|GetLobbyUI))
  (Utilities|IsValid _lobbyui
    (:Is%20Valid
      (Widget|RemovefromParent _lobbyui))))

(fn ConstructionScript)

(fn SetLobbyUI
  (params (UI :type WBP%20Lobby%20Object%20Reference))
  (bind _serverinfo (Variables|Default|GetServerInfo))
  (bind (_servername _maxplayers _map) (Utilities|Struct|BreakLobbyServerInfo _serverinfo))
  (Variables|Default|SetLobbyUI UI)
  (Variables|/Game/Frontier/Frontend/Lobby/WBP_Lobby.WBP_Lobby_C|SetServerName (Variables|Default|GetLobbyUI) (Utilities|Text|ToText(String) _servername))
  (Variables|/Game/Frontier/Frontend/Lobby/WBP_Lobby.WBP_Lobby_C|SetNumPlayers (Variables|Default|GetLobbyUI) _maxplayers)
  (Class|ComboBoxString|SetSelectedOption (Variables|/Game/Frontier/Frontend/Lobby/WBP_Lobby.WBP_Lobby_C|GetMapSelect (Variables|Default|GetLobbyUI)) _map))