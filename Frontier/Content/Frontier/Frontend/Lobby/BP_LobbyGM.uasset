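; BP_LobbyGM is the lobby game mode that tracks joining players, their ready states and server settings.
; On PostLogin it pulls server name and max players from the game instance, records the player and initializes their lobby controller.
; Join, ready and settings changes are pushed to every stored controller through parallel player and info arrays.
; StartGame server-travels to the map chosen in ServerInfo.
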(event Custom|SetPlayerReady
  (params (Player :type BP%20Lobby%20PC%20Object%20Reference) (Ready :type Boolean))
  (Utilities|Struct|SetmembersinLobbyPlayer (Utilities|Array|Get(acopy) (Variables|Default|GetPlayerInfos) (Utilities|Array|FindItem (Variables|Default|GetPlayers) Player)) Ready)
  (for _array_element (Variables|Default|GetPlayers)
    (Default|UpdatePlayerList _array_element (Variables|Default|GetPlayerInfos))))

(event Custom|StartGame
  (Development|ExecuteConsoleCommand (Utilities|String|Append "servertravel /Game/Frontier/Maps/" (.Map (Utilities|Struct|BreakLobbyServerInfo (Variables|Default|GetServerInfo)))) 0))

(event Custom|UpdateSettings
  (params (ServerInfo :type Lobby%20Server%20Info%20Structure))
  (Variables|Default|SetServerInfo ServerInfo)
  (for _array_element (Variables|Default|GetPlayers)
    (Default|UpdateServerInfo _array_element (Variables|Default|GetServerInfo))))

(event EventBeginPlay)

(event EventPostLogin
  (params (NewPlayer :type Player%20Controller%20Object%20Reference))
  (bind _players (Variables|Default|GetPlayers))
  (CallFunction|UpdateServerInfo)
  (bind _asbp_lobby_pc (Utilities|Casting|CastToBP_LobbyPC NewPlayer))
  (bind _asbp_lobby_ps (Utilities|Casting|CastToBP_LobbyPS (Variables|/Script/Engine.Controller|GetPlayerState _asbp_lobby_pc)))
  (Utilities|Array|Add (Variables|Default|GetPlayerInfos) (Utilities|Struct|MakeLobbyPlayer (Variables|/Script/Engine.PlayerState|GetPlayerName _asbp_lobby_ps) false))
  (Default|InitialSetup _asbp_lobby_pc)
  (Default|UpdateServerInfo _asbp_lobby_pc (Variables|Default|GetServerInfo))
  (Utilities|Array|Add _players _asbp_lobby_pc)
  (for _array_element _players
    (Default|UpdatePlayerList _array_element (Variables|Default|GetPlayerInfos))))

(fn ConstructionScript)

(fn UpdateServerInfo
  (bind _asbp_frontier_game_instance (Utilities|Casting|CastToBP_FrontierGameInstance (Game|GetGameInstance)))
  (Utilities|Struct|SetmembersinLobbyServerInfo (Variables|Default|GetServerInfo) (Variables|/Game/Frontier/Blueprints/BP_FrontierGameInstance.BP_FrontierGameInstance_C|GetServerName _asbp_frontier_game_instance) (Variables|/Game/Frontier/Blueprints/BP_FrontierGameInstance.BP_FrontierGameInstance_C|GetMaxPlayers _asbp_frontier_game_instance)))