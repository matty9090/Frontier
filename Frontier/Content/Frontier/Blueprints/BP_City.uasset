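; BP_City is a city actor that displays its name through a widget component.
; On BeginPlay it runs the parent logic, creates a WBP_CityName widget, assigns it to the CityNameWidget component and passes in CityName.
; The UpdateCityLabel event casts the component's widget and copies the current CityName into it to refresh the label.
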(event EventBeginPlay
  (|CallParentFunction)
  (bind _returnvalue (UserInterface|CreateWidget "/Game/Frontier/Blueprints/Widgets/WBP_CityName.WBP_CityName_C" (Game|GetPlayerController 0)))
  (UserInterface|SetWidget (Variables|Default|GetCityNameWidget) _returnvalue)
  (Variables|/Game/Frontier/Blueprints/Widgets/WBP_CityName.WBP_CityName_C|SetCityName _returnvalue (Variables|Default|GetCityName)))

(event EventUpdateCityLabel
  (bind _aswbp_city_name (Utilities|Casting|CastToWBP_CityName (UserInterface|GetUserWidgetObject (Variables|Default|GetCityNameWidget))))
  (Variables|/Game/Frontier/Blueprints/Widgets/WBP_CityName.WBP_CityName_C|SetCityName _aswbp_city_name (Variables|Default|GetCityName)))

(fn ConstructionScript)