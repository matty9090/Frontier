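; BP_BaseResource is a base actor for harvestable resources that holds a depletable ResourceAmount.
; Harvest subtracts the caller's GatherSpeed from that amount and returns how much was gathered.
; When the amount reaches zero or below, the actor destroys itself and returns only what remained, so the final harvest never overpays.
; The event graph and construction script are empty.
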(event EventBeginPlay)

(event Collision|EventActorBeginOverlap
  (params (OtherActor :type Actor%20Object%20Reference)))

(event EventTick
  (params (DeltaSeconds :type Float%20%28single-precision%29)))

(fn ConstructionScript)

(fn Harvest
  (params (GatherSpeed :type Integer))
  (bind _output_get (Variables|Default|SetResourceAmount (- (Variables|Default|GetResourceAmount) GatherSpeed)))
  (if (<= _output_get 0)
    (Actor|DestroyActor)
    (return (+ GatherSpeed (Variables|Default|GetResourceAmount)))
    (else
      (return GatherSpeed))))