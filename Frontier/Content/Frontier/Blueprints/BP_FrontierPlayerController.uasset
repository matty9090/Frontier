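; Player controller for an RTS-style game: creates the UI, pans and zooms the roam pawn, places buildings and commands units.
; Left-drag pans and the wheel zooms, both scaled by camera-height curves.
; A spawned building preview follows the cursor trace; left release passes its class and transform to ServerSpawnBuilding.
; Otherwise left release selects a FrontierCharacter, and right-click moves it through its AI controller.
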(event Custom|SetSelectedBuilding
  (params (BuildingType :type BP%20Building%20Class%20Reference))
  (Utilities|IsValid (Variables|Default|GetSelectedBuilding)
    (:Is%20Valid
      (Actor|DestroyActor (Variables|Default|GetSelectedBuilding)))
    (:Is%20Not%20Valid
      _))
  (bind _returnvalue (Game|SpawnActorfromClass BuildingType (Math|Transform|MakeTransform "0, 0, 0") "AdjustIfPossibleButAlwaysSpawn" 0 0))
  (Variables|Default|SetSelectedBuilding _returnvalue))

(event EventBeginPlay
  (bind _returnvalue (UserInterface|CreateWidget "/Game/Frontier/Blueprints/Widgets/WBP_UI.WBP_UI_C" self))
  (Utilities|IsValid _returnvalue
    (:Is%20Valid
      (UserInterface|Viewport|AddtoViewport _returnvalue 0))))

(event EventTick
  (params (DeltaSeconds :type Float%20%28single-precision%29))
  (bind _array (Utilities|Array|MakeArray "ObjectTypeQuery1"))
  (bind (_hitresult _returnvalue) (Class|PlayerController|GetHitResultUnderCursorforObjects _array true))
  (if (Variables|Default|GetIsDragging)
    (CallFunction|HandleDrag))
  (Utilities|IsValid (Variables|Default|GetSelectedBuilding)
    (:Is%20Valid
      (if _returnvalue
        (Transformation|SetActorLocation (Variables|Default|GetSelectedBuilding) (.Location (Collision|BreakHitResult _hitresult)) false true)))))

(event Input|MouseEvents|MouseWheelAxis
  (params (AxisValue :type Float%20%28single-precision%29))
  (bind _asbp_roam_pawn (Utilities|Casting|CastToBP_RoamPawn (Game|Player|GetPlayerPawn 0)))
  (bind _height (Default|GetCameraHeight _asbp_roam_pawn))
  (Default|SetCameraHeight _asbp_roam_pawn (Math|Float|Clamp(Float) (+ _height (* -1 (* AxisValue (* (Math|Curves|GetFloatValue (Variables|Default|GetZoomCurve) _height) (Variables|Default|GetZoomSpeed))))) (Variables|Default|GetMinZoom) (Variables|Default|GetMaxZoom))))

(event Input|MouseEvents|LeftMouseButton
  (params (Key :type Key%20Structure))
  (:Pressed
    (Utilities|IsValid (Variables|Default|GetSelectedBuilding)
      (:Is%20Not%20Valid
        (Variables|Default|SetIsDragging true))))
  (:Released
    (Variables|Default|SetIsDragging false)
    (Utilities|IsValid (Variables|Default|GetSelectedBuilding)
      (:Is%20Valid
        (CallFunction|PlaceBuilding))
      (:Is%20Not%20Valid
        (CallFunction|SelectUnit)))))

(event Input|MouseEvents|RightMouseButton
  (params (Key :type Key%20Structure))
  (:Pressed
    (CallFunction|SendUnittoLocation)))

(fn ConstructionScript)

(fn HandleDrag
  (bind (_deltax _deltay) (Class|PlayerController|GetInputMouseDelta))
  (bind _returnvalue (Game|Player|GetPlayerPawn 0))
  (bind _asbp_roam_pawn (Utilities|Casting|CastToBP_RoamPawn (Game|Player|GetPlayerPawn 0)))
  (bind _height (Default|GetCameraHeight _asbp_roam_pawn))
  (Transformation|SetActorLocation _returnvalue (+ (* (* (Math|Vector|MakeVector _deltay _deltax 0.0) -1) (* (Math|Curves|GetFloatValue (Variables|Default|GetMovementCurve) _height) (Variables|Default|GetMoveSpeed))) (Transformation|GetActorLocation _returnvalue)) false true))

(fn PlaceBuilding
  (bind _selectedbuilding (Variables|Default|GetSelectedBuilding))
  (Class|FrontierPlayerController|ServerSpawnBuilding (Utilities|GetClass _selectedbuilding) (Transformation|GetActorLocation _selectedbuilding) (Transformation|GetActorRotation _selectedbuilding)))

(fn SelectUnit
  (bind _array (Utilities|Array|MakeArray "ObjectTypeQuery3"))
  (bind (_hitresult _returnvalue) (Class|PlayerController|GetHitResultUnderCursorforObjects _array true))
  (if _returnvalue
    (bind _asbp_frontier_character (Utilities|Casting|CastToBP_FrontierCharacter (.HitActor (Collision|BreakHitResult _hitresult))))
    (Variables|Default|SetSelectedUnit _asbp_frontier_character)))

(fn SendUnittoLocation
  (bind _array (Utilities|Array|MakeArray "ObjectTypeQuery1" "ObjectTypeQuery2"))
  (bind (_hitresult _returnvalue) (Class|PlayerController|GetHitResultUnderCursorforObjects _array true))
  (Utilities|IsValid (Variables|Default|GetSelectedUnit)
    (:Is%20Valid
      (if _returnvalue
        (AI|Navigation|SimpleMovetoLocation (AI|GetAIController (Variables|Default|GetSelectedUnit)) (.ImpactPoint (Collision|BreakHitResult _hitresult)))))))