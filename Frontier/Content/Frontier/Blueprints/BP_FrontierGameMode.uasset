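; Frontier game mode that assigns player starts and sets up each player at the assigned location.
; ChoosePlayerStart takes the first spot from a cached PlayerStart list and removes it, refilling the list from the level when empty so starts are handed out in rotation.
; InitStartSpot passes the player and the start spot's location to SetupPlayer, which is defined outside this graph.
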(event EventBeginPlay)

(event EventInitStartSpot
  (params (StartSpot :type Actor%20Object%20Reference) (NewPlayer :type Controller%20Object%20Reference))
  (Class|FrontierGameMode|SetupPlayer NewPlayer (Transformation|GetActorLocation StartSpot)))

(fn ConstructionScript)

(fn ChoosePlayerStart
  (params (Player :type Controller%20Object%20Reference))
  (if (<= (Utilities|Array|Length (Variables|Default|GetStartSpots)) 0)
    (bind _outactors (Actor|GetAllActorsOfClass "/Script/Engine.PlayerStart"))
    (Variables|Default|SetStartSpots _outactors))
  (bind _output_get (LocalVariables|SetSpot (Utilities|Array|Get(acopy) (Variables|Default|GetStartSpots))))
  (Utilities|Array|RemoveIndex (Variables|Default|GetStartSpots))
  (return _output_get))