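; Blueprint function library of UI helpers for Frontier, currently holding a single button styling function.
; CreateButtonStyle builds a button style from box brush assets and applies it to the given button.
; Clickable buttons get distinct hovered and pressed brushes, while non-clickable ones keep the normal brush for those states.
; Both variants share the same disabled brush, and the button's enabled state is left untouched.
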(fn CreateButtonStyle
  (params (Button :type Button%20Object%20Reference) (Clickable :type Boolean))
  (if Clickable
    (Class|Button|SetStyle Button (Utilities|Struct|MakeButtonStyle (Class|WidgetBlueprintLibrary|MakeBrushfromAsset "/Game/Frontier/Brushes/Brush_Box.Brush_Box") (Class|WidgetBlueprintLibrary|MakeBrushfromAsset "/Game/Frontier/Brushes/Brush_Box2.Brush_Box2") (Class|WidgetBlueprintLibrary|MakeBrushfromAsset "/Game/Frontier/Brushes/Brush_Box4.Brush_Box4") (Class|WidgetBlueprintLibrary|MakeBrushfromAsset "/Game/Frontier/Brushes/Brush_Box4.Brush_Box4")))
    (else
      (Class|Button|SetStyle Button (Utilities|Struct|MakeButtonStyle (Class|WidgetBlueprintLibrary|MakeBrushfromAsset "/Game/Frontier/Brushes/Brush_Box.Brush_Box") (Class|WidgetBlueprintLibrary|MakeBrushfromAsset "/Game/Frontier/Brushes/Brush_Box.Brush_Box") (Class|WidgetBlueprintLibrary|MakeBrushfromAsset "/Game/Frontier/Brushes/Brush_Box.Brush_Box") (Class|WidgetBlueprintLibrary|MakeBrushfromAsset "/Game/Frontier/Brushes/Brush_Box4.Brush_Box4"))))))