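; BP_FrontierPlayerState is the player state for Frontier, defining the research tree through CreateResearchTree.
; It creates a pre-researched Civilisation root holding the starting buildings and worker, then chains AddChild calls for costed Fighting and Architechture branches that list further buildings.
; Fighting continues into placeholder "Idk" and "Stuff" nodes, and the function returns the root.
; BeginPlay and the construction script are empty.
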(event EventBeginPlay)

(fn ConstructionScript)

(fn CreateResearchTree
  (bind _returnvalue (Class|FrontierHelperFunctionLibrary|CreateResources 100))
  (bind _returnvalue_2 (Class|FrontierHelperFunctionLibrary|CreateResources 0 100))
  (bind _array (Utilities|Array|MakeArray 0))
  (bind _returnvalue_3 (Class|FrontierHelperFunctionLibrary|CreateResearchNode "Civilisation" (Class|FrontierHelperFunctionLibrary|CreateResources) (Utilities|Array|MakeArray "/Game/Frontier/Blueprints/Buildings/TownHall/BP_TownHall.BP_TownHall_C" "/Game/Frontier/Blueprints/Units/BP_Worker.BP_Worker_C" "/Game/Frontier/Blueprints/Buildings/Library/BP_Library.BP_Library_C" "/Game/Frontier/Blueprints/Buildings/Storage/BP_Storage.BP_Storage_C" "/Game/Frontier/Blueprints/Buildings/House/BP_House.BP_House_C") "Researched" 0 self))
  (Utilities|FlowControl|Sequence
    (:then_0
      (bind _returnvalue_4 (Class|ResearchNode|AddChild _returnvalue_3 "Fighting" _returnvalue (Utilities|Array|MakeArray "/Game/Frontier/Blueprints/Buildings/Barracks/BP_Barracks.BP_Barracks_C" "/Game/Frontier/Blueprints/Buildings/Turret/BP_Turret.BP_Turret_C"))))
    (:then_1
      (Class|ResearchNode|AddChild _returnvalue_3 "Architechture" _returnvalue (Utilities|Array|MakeArray "/Game/Frontier/Blueprints/Buildings/Library/BP_Library.BP_Library_C" "/Game/Frontier/Blueprints/Buildings/Stable/BP_Stable.BP_Stable_C"))
      (bind _returnvalue_5 (Class|ResearchNode|AddChild _returnvalue_4 "Idk" _returnvalue_2 (Utilities|Array|MakeArray 0)))
      (Utilities|FlowControl|Sequence
        (:then_0
          (Class|ResearchNode|AddChild _returnvalue_5 "Stuff" _returnvalue_2 _array))
        (:then_1
          (Class|ResearchNode|AddChild _returnvalue_5 "Stuff" _returnvalue_2 _array))
        (:then_2
          (Class|ResearchNode|AddChild _returnvalue_5 "Stuff" _returnvalue_2 _array))
        (:then_3
          (return _returnvalue_3))))))